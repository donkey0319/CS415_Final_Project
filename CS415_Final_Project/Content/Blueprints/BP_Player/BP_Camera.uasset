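; BP_Camera is a side-on shared camera that keeps two players framed by following the midpoint between them on X and Z.
; Each Tick re-finds both BP_Player1 actors, Player2 by tag and Player1 as the first of the class.
; Camera Y grows with their horizontal separation, with a minimum offset from Player1's initial Y, and holds when separation is zero.
; The actor moves there with a swept transform at fixed rotation.
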(event EventBeginPlay)

(event Collision|EventActorBeginOverlap
  (params (OtherActor :type Actor%20Object%20Reference)))

(event EventTick
  (params (DeltaSeconds :type Float%20%28single-precision%29))
  (bind _player1 (Variables|Default|GetPlayer1))
  (bind _player2 (Variables|Default|GetPlayer2))
  (bind _returnvalue (Transformation|GetActorLocation _player2))
  (bind _returnvalue_2 (Transformation|GetActorLocation _player1))
  (bind _returnvalue_3 (- (.x _returnvalue_2) (.x _returnvalue)))
  (bind _returnvalue_4 (Math|Float|Absolute(Float) _returnvalue_3))
  (CallFunction|SetPlayer1and2)
  (Utilities|FlowControl|Sequence
    (:then_0
      (if (!= 0.0 _returnvalue_4)
        (Variables|Default|SetCamera_y (Math|Float|Max(Float) (/ _returnvalue_4 (- 1.0 (/ 0.36 _returnvalue_4))) (+ (Variables|/Game/Blueprints/BP_Player/BP_Player1.BP_Player1_C|Getinitial%20y-location (Variables|Default|GetPlayer1)) 1e+03)))
        (else
          (Variables|Default|SetCamera_y (.y (.location (Transformation|GetWorldTransform (Variables|Default|GetCamera))))))))
    (:then_1
      (Transformation|SetActorTransform (Math|Transform|MakeTransform (Math|Vector|MakeVector (/ (+ (.x _returnvalue_2) (.x _returnvalue)) 2.0) (Variables|Default|GetCamera_y) (/ (+ (.z _returnvalue_2) (.z _returnvalue)) 2.0)) "0.000000,-90.000000,0.000000" "1.000000,1.000000,1.000000") true))))

(fn ConstructionScript)

(fn SetPlayer1and2
  (bind _outactors (Actor|GetAllActorswithTag "Player2"))
  (bind _asbp_player_1 (Utilities|Casting|CastToBP_Player1 (Utilities|Array|Get(acopy) _outactors)))
  (Variables|Default|SetPlayer2 _asbp_player_1)
  (bind _outactors_2 (Actor|GetAllActorsOfClass "/Game/Blueprints/BP_Player/BP_Player1.BP_Player1_C"))
  (Variables|Default|SetPlayer1 (Utilities|Array|Get(acopy) _outactors_2)))